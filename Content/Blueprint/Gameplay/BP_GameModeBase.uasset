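; Game mode that runs a single round of blackjack between the player and a dealer.
; After a short delay it caches ten pre-placed card actors and their values, then totals the opening hands.
; Separate Hit and DealerTurn functions reveal cards, add values and, in some cases, count aces as one on a bust.
; Compare prints win, draw or lose, with the dealer drawing on 16 or less.
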(event Custom|PlayerHand
  (Variables|Default|SetPlayer (+ (Variables|Default|GetCard) (Variables|Default|GetCard1)))
  (if (> (Variables|Default|GetPlayer) 21)
    (Variables|Default|SetPlayer (- (Variables|Default|GetPlayer) 10))
    (Variables|/Game/Blueprint/Card/BP_Card.BP_Card_C|SetACE (Variables|Default|GetBPCard) false)))

(event Custom|EnemyHand
  (Variables|Default|SetEnemy (Variables|Default|GetCard3)))

(event EventBeginPlay
  (Utilities|FlowControl|Delay 1.0)
  (CallFunction|SetValue)
  (CallFunction|PlayerHand)
  (CallFunction|EnemyHand))

(fn ConstructionScript)

(fn SetValue
  (Utilities|FlowControl|Sequence
    (:then_0
      (bind _returnvalue (Actor|GetActorOfClass "/Game/Blueprint/Card/BP_Card.BP_Card_C"))
      (Variables|Default|SetCard (Variables|/Game/Blueprint/Card/BP_Card.BP_Card_C|GetValue _returnvalue))
      (Variables|Default|SetBPCard _returnvalue))
    (:then_1
      (bind _returnvalue_2 (Actor|GetActorOfClass "/Game/Blueprint/Card/BP_Card1.BP_Card1_C"))
      (Variables|Default|SetCard1 (Variables|/Game/Blueprint/Card/BP_Card1.BP_Card1_C|GetValue _returnvalue_2))
      (Variables|Default|SetBPCard1 _returnvalue_2))
    (:then_2
      (bind _returnvalue_3 (Actor|GetActorOfClass "/Game/Blueprint/Card/BP_Card2.BP_Card2_C"))
      (Variables|Default|SetCard2 (Variables|/Game/Blueprint/Card/BP_Card2.BP_Card2_C|GetValue _returnvalue_3))
      (Variables|Default|SetBPCard2 _returnvalue_3))
    (:then_3
      (bind _returnvalue_4 (Actor|GetActorOfClass "/Game/Blueprint/Card/BP_Card3.BP_Card3_C"))
      (Variables|Default|SetCard3 (Variables|/Game/Blueprint/Card/BP_Card3.BP_Card3_C|GetValue _returnvalue_4))
      (Variables|Default|SetBPCard3 _returnvalue_4))
    (:then_4
      (bind _returnvalue_5 (Actor|GetActorOfClass "/Game/Blueprint/Card/BP_Card4.BP_Card4_C"))
      (Variables|Default|SetCard4 (Variables|/Game/Blueprint/Card/BP_Card4.BP_Card4_C|GetValue _returnvalue_5))
      (Variables|Default|SetBPCard4 _returnvalue_5))
    (:then_5
      (bind _returnvalue_6 (Actor|GetActorOfClass "/Game/Blueprint/Card/BP_Card5.BP_Card5_C"))
      (Variables|Default|SetCard5 (Variables|/Game/Blueprint/Card/BP_Card5.BP_Card5_C|GetValue _returnvalue_6))
      (Variables|Default|SetBPCard5 _returnvalue_6))
    (:then_6
      (bind _returnvalue_7 (Actor|GetActorOfClass "/Game/Blueprint/Card/BP_Card6.BP_Card6_C"))
      (Variables|Default|SetCard6 (Variables|/Game/Blueprint/Card/BP_Card6.BP_Card6_C|GetValue _returnvalue_7))
      (Variables|Default|SetBPCard6 _returnvalue_7))
    (:then_7
      (bind _returnvalue_8 (Actor|GetActorOfClass "/Game/Blueprint/Card/BP_Card7.BP_Card7_C"))
      (Variables|Default|SetCard7 (Variables|/Game/Blueprint/Card/BP_Card7.BP_Card7_C|GetValue _returnvalue_8))
      (Variables|Default|SetBPCard7 _returnvalue_8))
    (:then_8
      (bind _returnvalue_9 (Actor|GetActorOfClass "/Game/Blueprint/Card/BP_Card8.BP_Card8_C"))
      (Variables|Default|SetCard8 (Variables|/Game/Blueprint/Card/BP_Card8.BP_Card8_C|GetValue _returnvalue_9))
      (Variables|Default|SetBPCard8 _returnvalue_9))
    (:then_9
      (bind _returnvalue_10 (Actor|GetActorOfClass "/Game/Blueprint/Card/BP_Card9.BP_Card9_C"))
      (Variables|Default|SetCard9 (Variables|/Game/Blueprint/Card/BP_Card9.BP_Card9_C|GetValue _returnvalue_10))
      (Variables|Default|SetBPCard9 _returnvalue_10))))

(fn Compare
  (if (> (Variables|Default|GetEnemy) 21)
    (Development|PrintString "Win")
    (elif (> (Variables|Default|GetPlayer) (Variables|Default|GetEnemy))
      (Development|PrintString "Win")
      (elif (== (Variables|Default|GetPlayer) (Variables|Default|GetEnemy))
        (Development|PrintString "Draw")
        (elif (< (Variables|Default|GetPlayer) (Variables|Default|GetEnemy))
          (Development|PrintString "Lose"))))))

(fn DealerTurn1
  (Variables|Default|SetReveal true)
  (Transformation|SetActorRotation (Variables|Default|GetBPCard2) "180.000000, 0, 0")
  (Variables|Default|SetEnemy (+ (Variables|Default|GetEnemy) (Variables|Default|GetCard2)))
  (if (> (Variables|Default|GetEnemy) 21)
    (Variables|Default|SetEnemy (- (Variables|Default|GetEnemy) 10))
    (Variables|/Game/Blueprint/Card/BP_Card2.BP_Card2_C|SetACE (Variables|Default|GetBPCard2) false)))

(fn Hit
  (Transformation|SetActorLocation (Variables|Default|GetBPCard4) "15.500000,23.760799,115.965591" false false)
  (Transformation|SetActorRotation (Variables|Default|GetBPCard4) "180.000000, 0, 0")
  (Rendering|SetActorHiddenInGame (Variables|Default|GetBPCard4) false)
  (Variables|Default|SetPlayer (+ (Variables|Default|GetPlayer) (Variables|Default|GetCard4)))
  (if (> (Variables|Default|GetPlayer) 21)
    (if (Variables|/Game/Blueprint/Card/BP_Card4.BP_Card4_C|GetACE (Variables|Default|GetBPCard4))
      (Variables|Default|SetPlayer (- (Variables|Default|GetPlayer) 10))
      (Variables|/Game/Blueprint/Card/BP_Card4.BP_Card4_C|SetACE (Variables|Default|GetBPCard4) false)
      (elif (and (Variables|/Game/Blueprint/Card/BP_Card.BP_Card_C|GetACE (Variables|Default|GetBPCard)) (> (Variables|Default|GetPlayer) 21))
        (Variables|Default|SetPlayer (- (Variables|Default|GetPlayer) 10))
        (Variables|/Game/Blueprint/Card/BP_Card.BP_Card_C|SetACE (Variables|Default|GetBPCard) false)
        (elif (and (Variables|/Game/Blueprint/Card/BP_Card1.BP_Card1_C|GetACE (Variables|Default|GetBPCard1)) (> (Variables|Default|GetPlayer) 21))
          (Variables|Default|SetPlayer (- (Variables|Default|GetPlayer) 10))
          (Variables|/Game/Blueprint/Card/BP_Card1.BP_Card1_C|SetACE (Variables|Default|GetBPCard1) false)
          (else
            (Development|PrintString "Lose")))))))

(fn Hit2
  (Transformation|SetActorLocation (Variables|Default|GetBPCard5) "23.500000,23.760799,115.965591" false false)
  (Transformation|SetActorRotation (Variables|Default|GetBPCard5) "180.000000, 0, 0")
  (Rendering|SetActorHiddenInGame (Variables|Default|GetBPCard5) false)
  (Variables|Default|SetPlayer (+ (Variables|Default|GetPlayer) (Variables|Default|GetCard5)))
  (if (> (Variables|Default|GetPlayer) 21)
    (if (Variables|/Game/Blueprint/Card/BP_Card4.BP_Card4_C|GetACE (Variables|Default|GetBPCard4))
      (Variables|Default|SetPlayer (- (Variables|Default|GetPlayer) 10))
      (Variables|/Game/Blueprint/Card/BP_Card4.BP_Card4_C|SetACE (Variables|Default|GetBPCard4) false)
      (elif (and (Variables|/Game/Blueprint/Card/BP_Card.BP_Card_C|GetACE (Variables|Default|GetBPCard)) (> (Variables|Default|GetPlayer) 21))
        (Variables|Default|SetPlayer (- (Variables|Default|GetPlayer) 10))
        (Variables|/Game/Blueprint/Card/BP_Card.BP_Card_C|SetACE (Variables|Default|GetBPCard) false)
        (elif (and (Variables|/Game/Blueprint/Card/BP_Card1.BP_Card1_C|GetACE (Variables|Default|GetBPCard1)) (> (Variables|Default|GetPlayer) 21))
          (Variables|Default|SetPlayer (- (Variables|Default|GetPlayer) 10))
          (Variables|/Game/Blueprint/Card/BP_Card1.BP_Card1_C|SetACE (Variables|Default|GetBPCard1) false)
          (elif (and (Variables|/Game/Blueprint/Card/BP_Card5.BP_Card5_C|GetACE (Variables|Default|GetBPCard5)) (> (Variables|Default|GetPlayer) 21))
            (Variables|Default|SetPlayer (- (Variables|Default|GetPlayer) 10))
            (Variables|/Game/Blueprint/Card/BP_Card5.BP_Card5_C|SetACE (Variables|Default|GetBPCard5) false)
            (else
              (Development|PrintString "Lose"))))))))

(fn Hit3
  (Transformation|SetActorLocation (Variables|Default|GetBPCard6) "31.500000,23.760799,115.965591" false false)
  (Transformation|SetActorRotation (Variables|Default|GetBPCard6) "180.000000, 0, 0")
  (Rendering|SetActorHiddenInGame (Variables|Default|GetBPCard6) false)
  (Variables|Default|SetPlayer (+ (Variables|Default|GetPlayer) (Variables|Default|GetCard6)))
  (if (> (Variables|Default|GetPlayer) 21)
    (if (Variables|/Game/Blueprint/Card/BP_Card4.BP_Card4_C|GetACE (Variables|Default|GetBPCard4))
      (Variables|Default|SetPlayer (- (Variables|Default|GetPlayer) 10))
      (Variables|/Game/Blueprint/Card/BP_Card4.BP_Card4_C|SetACE (Variables|Default|GetBPCard4) false)
      (elif (and (Variables|/Game/Blueprint/Card/BP_Card.BP_Card_C|GetACE (Variables|Default|GetBPCard)) (> (Variables|Default|GetPlayer) 21))
        (Variables|Default|SetPlayer (- (Variables|Default|GetPlayer) 10))
        (Variables|/Game/Blueprint/Card/BP_Card.BP_Card_C|SetACE (Variables|Default|GetBPCard) false)
        (elif (and (Variables|/Game/Blueprint/Card/BP_Card1.BP_Card1_C|GetACE (Variables|Default|GetBPCard1)) (> (Variables|Default|GetPlayer) 21))
          (Variables|Default|SetPlayer (- (Variables|Default|GetPlayer) 10))
          (Variables|/Game/Blueprint/Card/BP_Card1.BP_Card1_C|SetACE (Variables|Default|GetBPCard1) false)
          (elif (and (Variables|/Game/Blueprint/Card/BP_Card5.BP_Card5_C|GetACE (Variables|Default|GetBPCard5)) (> (Variables|Default|GetPlayer) 21))
            (Variables|Default|SetPlayer (- (Variables|Default|GetPlayer) 10))
            (Variables|/Game/Blueprint/Card/BP_Card5.BP_Card5_C|SetACE (Variables|Default|GetBPCard5) false)
            (elif (and (Variables|/Game/Blueprint/Card/BP_Card6.BP_Card6_C|GetACE (Variables|Default|GetBPCard6)) (> (Variables|Default|GetPlayer) 21))
              (Variables|Default|SetPlayer (- (Variables|Default|GetPlayer) 10))
              (Variables|/Game/Blueprint/Card/BP_Card6.BP_Card6_C|SetACE (Variables|Default|GetBPCard6) false)
              (else
                (Development|PrintString "Lose")))))))
    (else
      (CallFunction|Compare))))

(fn DealerTurn2
  (if (<= (Variables|Default|GetEnemy) 16)
    (Transformation|SetActorLocation (Variables|Default|GetBPCard7) "15.500000,2.000000,116.400002" false false)
    (Transformation|SetActorRotation (Variables|Default|GetBPCard7) "180.000000, 0, 0")
    (Rendering|SetActorHiddenInGame (Variables|Default|GetBPCard7) false)
    (Variables|Default|SetEnemy (+ (Variables|Default|GetEnemy) (Variables|Default|GetCard7)))
    (else
      (CallFunction|Compare))))

(fn DealerTurn3
  (if (<= (Variables|Default|GetEnemy) 16)
    (Transformation|SetActorLocation (Variables|Default|GetBPCard8) "23.500000,2.000000,116.400002" false false)
    (Transformation|SetActorRotation (Variables|Default|GetBPCard8) "180.000000, 0, 0")
    (Rendering|SetActorHiddenInGame (Variables|Default|GetBPCard8) false)
    (Variables|Default|SetEnemy (+ (Variables|Default|GetEnemy) (Variables|Default|GetCard8)))
    (else
      (CallFunction|Compare))))

(fn DealerTurn4
  (if (<= (Variables|Default|GetEnemy) 16)
    (Transformation|SetActorLocation (Variables|Default|GetBPCard9) "31.500000,2.000000,116.400002" false false)
    (Transformation|SetActorRotation (Variables|Default|GetBPCard9) "180.000000, 0, 0")
    (Rendering|SetActorHiddenInGame (Variables|Default|GetBPCard9) false)
    (Variables|Default|SetEnemy (+ (Variables|Default|GetEnemy) (Variables|Default|GetCard9)))
    (CallFunction|Compare)
    (else
      (CallFunction|Compare))))