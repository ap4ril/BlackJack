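; BP_HitButton is a clickable Hit button actor, likely for a card game such as blackjack, that shifts slightly on cursor hover.
; It stays hidden for about ten seconds after BeginPlay.
; Releases use a counter to call Hit, Hit2, then Hit3 on BP_GameModeBase, repeating Hit3 thereafter.
; Each press runs one of three identical HideButton graphs, hiding it and BP_StandButton for five seconds.
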(event OnBeginCursorOver(HitButton)
  (params (TouchedComponent :type Primitive%20Component%20Object%20Reference))
  (Variables|Default|SetLocation "0, 0,-1.000000")
  (Transformation|AddLocalOffset (Variables|Default|GetHitButton) (Variables|Default|GetLocation) false false))

(event OnEndCursorOver(HitButton)
  (params (TouchedComponent :type Primitive%20Component%20Object%20Reference))
  (Variables|Default|SetLocation "0, 0,1.000000")
  (Transformation|AddLocalOffset (Variables|Default|GetHitButton) (Variables|Default|GetLocation) false false))

(event OnReleased(HitButton)
  (params (TouchedComponent :type Primitive%20Component%20Object%20Reference) (ButtonReleased :type Key%20Structure :default "None"))
  (switch int (Variables|Default|GetCount)
    (:0
      (Default|Hit (Variables|Default|GetGameMode))
      (Math|Integer|IncrementInt (Variables|Default|GetCount)
        (:%20%20
          (|HideButton))))
    (:1
      (Default|Hit2 (Variables|Default|GetGameMode))
      (Math|Integer|IncrementInt (Variables|Default|GetCount)
        (:%20%20
          (|HideButton_2))))
    (:2
      (Default|Hit3 (Variables|Default|GetGameMode))
      (|HideButton_2_2))))

(event EventBeginPlay
  (bind _asbp_game_mode_base (Utilities|Casting|CastToBP_GameModeBase (Game|GetGameMode)))
  (Variables|Default|SetGameMode _asbp_game_mode_base)
  (Rendering|SetActorHiddenInGame true)
  (Utilities|FlowControl|Delay 10.3)
  (Rendering|SetActorHiddenInGame false)
  (Variables|Default|SetCount 0))

(event Collision|EventActorBeginOverlap
  (params (OtherActor :type Actor%20Object%20Reference)))

(event EventTick
  (params (DeltaSeconds :type Float%20%28single-precision%29)))

(fn ConstructionScript)