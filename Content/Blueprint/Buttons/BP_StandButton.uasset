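; Clickable 3D Stand button that triggers the dealer's turns on the game mode when released.
; It caches BP_GameModeBase on BeginPlay and stays hidden until a startup delay elapses.
; Cursor hover nudges the StandButton component down by a local Z offset and back up on exit.
; Release calls DealerTurn1 through DealerTurn4 in sequence, spaced by fixed delays rather than completion callbacks.
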(event OnBeginCursorOver(StandButton)
  (params (TouchedComponent :type Primitive%20Component%20Object%20Reference))
  (Variables|Default|SetLocation "0, 0,-1.000000")
  (Transformation|AddLocalOffset (Variables|Default|GetStandButton) (Variables|Default|GetLocation) false false))

(event OnEndCursorOver(StandButton)
  (params (TouchedComponent :type Primitive%20Component%20Object%20Reference))
  (Variables|Default|SetLocation "0, 0,1.000000")
  (Transformation|AddLocalOffset (Variables|Default|GetStandButton) (Variables|Default|GetLocation) false false))

(event OnReleased(StandButton)
  (params (TouchedComponent :type Primitive%20Component%20Object%20Reference) (ButtonReleased :type Key%20Structure :default "None"))
  (Default|DealerTurn1 (Variables|Default|GetGameMode))
  (Utilities|FlowControl|Delay 2.0)
  (Default|DealerTurn2 (Variables|Default|GetGameMode))
  (Utilities|FlowControl|Delay 4.0)
  (Default|DealerTurn3 (Variables|Default|GetGameMode))
  (Utilities|FlowControl|Delay 4.0)
  (Default|DealerTurn4 (Variables|Default|GetGameMode)))

(event EventBeginPlay
  (bind _asbp_game_mode_base (Utilities|Casting|CastToBP_GameModeBase (Game|GetGameMode)))
  (Variables|Default|SetGameMode _asbp_game_mode_base)
  (Rendering|SetActorHiddenInGame true)
  (Utilities|FlowControl|Delay 10.3)
  (Rendering|SetActorHiddenInGame false))

(event Collision|EventActorBeginOverlap
  (params (OtherActor :type Actor%20Object%20Reference)))

(event EventTick
  (params (DeltaSeconds :type Float%20%28single-precision%29)))

(fn ConstructionScript)