(event EventTick
  (params (DeltaSeconds :type Float%20%28single-precision%29))
  (if (Variables|/Game/Blueprint/Dealer/BP_Dealer.BP_Dealer_C|GetCircle7 (Variables|Default|GetDealer))
    (Rendering|SetActorHiddenInGame false)
    (Transformation|SetActorRotation "0, 0,45.000000")
    (|Circular DeltaSeconds)))

(event EventBeginPlay
  (bind _returnvalue (Actor|GetActorOfClass "/Game/Blueprint/Dealer/BP_Dealer.BP_Dealer_C"))
  (Variables|Default|SetDealer _returnvalue)
  (Rendering|SetActorHiddenInGame true)
  (bind _asbp_game_mode_base (Utilities|Casting|CastToBP_GameModeBase (Game|GetGameMode)))
  (Variables|Default|SetGameMode _asbp_game_mode_base))

(fn ConstructionScript)

(fn MakeArray
  (Utilities|FlowControl|Sequence
    (:then_0
      (bind _output_get (Variables|Default|SetS1 "/Game/Casino/Models/PlayingCards/Spade/SM_PC01s.SM_PC01s")))
    (:then_1
      (bind _output_get_2 (Variables|Default|SetS2 "/Game/Casino/Models/PlayingCards/Spade/SM_PC02s.SM_PC02s")))
    (:then_2
      (bind _output_get_3 (Variables|Default|SetS3 "/Game/Casino/Models/PlayingCards/Spade/SM_PC03s.SM_PC03s")))
    (:then_3
      (bind _output_get_4 (Variables|Default|SetS4 "/Game/Casino/Models/PlayingCards/Spade/SM_PC04s.SM_PC04s")))
    (:then_4
      (bind _output_get_5 (Variables|Default|SetS5 "/Game/Casino/Models/PlayingCards/Spade/SM_PC05s.SM_PC05s")))
    (:then_5
      (bind _output_get_6 (Variables|Default|SetS6 "/Game/Casino/Models/PlayingCards/Spade/SM_PC06s.SM_PC06s")))
    (:then_6
      (bind _output_get_7 (Variables|Default|SetS7 "/Game/Casino/Models/PlayingCards/Spade/SM_PC07s.SM_PC07s")))
    (:then_7
      (bind _output_get_8 (Variables|Default|SetS8 "/Game/Casino/Models/PlayingCards/Spade/SM_PC08s.SM_PC08s")))
    (:then_8
      (bind _output_get_9 (Variables|Default|SetS9 "/Game/Casino/Models/PlayingCards/Spade/SM_PC09s.SM_PC09s")))
    (:then_9
      (bind _output_get_10 (Variables|Default|SetS10 "/Game/Casino/Models/PlayingCards/Spade/SM_PC10s.SM_PC10s")))
    (:then_10
      (bind _output_get_11 (Variables|Default|SetSJ "/Game/Casino/Models/PlayingCards/Spade/SM_PC11s.SM_PC11s")))
    (:then_11
      (bind _output_get_12 (Variables|Default|SetSQ "/Game/Casino/Models/PlayingCards/Spade/SM_PC12s.SM_PC12s")))
    (:then_12
      (bind _output_get_13 (Variables|Default|SetSK "/Game/Casino/Models/PlayingCards/Spade/SM_PC13s.SM_PC13s"))))
  (Variables|Default|SetS (Utilities|Array|MakeArray _output_get _output_get_2 _output_get_3 _output_get_4 _output_get_5 _output_get_6 _output_get_7 _output_get_8 _output_get_9 _output_get_10 _output_get_11 _output_get_12 _output_get_13))
  (Utilities|FlowControl|Sequence
    (:then_0
      (bind _output_get_14 (Variables|Default|SetC1 "/Game/Casino/Models/PlayingCards/Club/SM_PC01c.SM_PC01c")))
    (:then_1
      (bind _output_get_15 (Variables|Default|SetC2 "/Game/Casino/Models/PlayingCards/Club/SM_PC02c.SM_PC02c")))
    (:then_2
      (bind _output_get_16 (Variables|Default|SetC3 "/Game/Casino/Models/PlayingCards/Club/SM_PC03c.SM_PC03c")))
    (:then_3
      (bind _output_get_17 (Variables|Default|SetC4 "/Game/Casino/Models/PlayingCards/Club/SM_PC04c.SM_PC04c")))
    (:then_4
      (bind _output_get_18 (Variables|Default|SetC5 "/Game/Casino/Models/PlayingCards/Club/SM_PC05c.SM_PC05c")))
    (:then_5
      (bind _output_get_19 (Variables|Default|SetC6 "/Game/Casino/Models/PlayingCards/Club/SM_PC06c.SM_PC06c")))
    (:then_6
      (bind _output_get_20 (Variables|Default|SetC7 "/Game/Casino/Models/PlayingCards/Club/SM_PC07c.SM_PC07c")))
    (:then_7
      (bind _output_get_21 (Variables|Default|SetC8 "/Game/Casino/Models/PlayingCards/Club/SM_PC08c.SM_PC08c")))
    (:then_8
      (bind _output_get_22 (Variables|Default|SetC9 "/Game/Casino/Models/PlayingCards/Club/SM_PC09c.SM_PC09c")))
    (:then_9
      (bind _output_get_23 (Variables|Default|SetC10 "/Game/Casino/Models/PlayingCards/Club/SM_PC10c.SM_PC10c")))
    (:then_10
      (bind _output_get_24 (Variables|Default|SetC11 "/Game/Casino/Models/PlayingCards/Club/SM_PC11c.SM_PC11c")))
    (:then_11
      (bind _output_get_25 (Variables|Default|SetC12 "/Game/Casino/Models/PlayingCards/Club/SM_PC12c.SM_PC12c")))
    (:then_12
      (bind _output_get_26 (Variables|Default|SetC13 "/Game/Casino/Models/PlayingCards/Club/SM_PC13c.SM_PC13c"))))
  (Variables|Default|SetC (Utilities|Array|MakeArray _output_get_14 _output_get_15 _output_get_16 _output_get_17 _output_get_18 _output_get_19 _output_get_20 _output_get_21 _output_get_22 _output_get_23 _output_get_24 _output_get_25 _output_get_26))
  (Utilities|FlowControl|Sequence
    (:then_0
      (bind _output_get_27 (Variables|Default|SetD1 "/Game/Casino/Models/PlayingCards/Diamond/SM_PC01d.SM_PC01d")))
    (:then_1
      (bind _output_get_28 (Variables|Default|SetD2 "/Game/Casino/Models/PlayingCards/Diamond/SM_PC02d.SM_PC02d")))
    (:then_2
      (bind _output_get_29 (Variables|Default|SetD3 "/Game/Casino/Models/PlayingCards/Diamond/SM_PC03d.SM_PC03d")))
    (:then_3
      (bind _output_get_30 (Variables|Default|SetD4 "/Game/Casino/Models/PlayingCards/Diamond/SM_PC04d.SM_PC04d")))
    (:then_4
      (bind _output_get_31 (Variables|Default|SetD5 "/Game/Casino/Models/PlayingCards/Diamond/SM_PC05d.SM_PC05d")))
    (:then_5
      (bind _output_get_32 (Variables|Default|SetD6 "/Game/Casino/Models/PlayingCards/Diamond/SM_PC06d.SM_PC06d")))
    (:then_6
      (bind _output_get_33 (Variables|Default|SetD7 "/Game/Casino/Models/PlayingCards/Diamond/SM_PC07d.SM_PC07d")))
    (:then_7
      (bind _output_get_34 (Variables|Default|SetD8 "/Game/Casino/Models/PlayingCards/Diamond/SM_PC08d.SM_PC08d")))
    (:then_8
      (bind _output_get_35 (Variables|Default|SetD9 "/Game/Casino/Models/PlayingCards/Diamond/SM_PC09d.SM_PC09d")))
    (:then_9
      (bind _output_get_36 (Variables|Default|SetD10 "/Game/Casino/Models/PlayingCards/Diamond/SM_PC10d.SM_PC10d")))
    (:then_10
      (bind _output_get_37 (Variables|Default|SetDJ "/Game/Casino/Models/PlayingCards/Diamond/SM_PC11d.SM_PC11d")))
    (:then_11
      (bind _output_get_38 (Variables|Default|SetDQ "/Game/Casino/Models/PlayingCards/Diamond/SM_PC12d.SM_PC12d")))
    (:then_12
      (bind _output_get_39 (Variables|Default|SetDK "/Game/Casino/Models/PlayingCards/Diamond/SM_PC13d.SM_PC13d"))))
  (Variables|Default|SetD (Utilities|Array|MakeArray _output_get_27 _output_get_28 _output_get_29 _output_get_30 _output_get_31 _output_get_32 _output_get_33 _output_get_34 _output_get_35 _output_get_36 _output_get_37 _output_get_38 _output_get_39))
  (Utilities|FlowControl|Sequence
    (:then_0
      (bind _output_get_40 (Variables|Default|SetH1 "/Game/Casino/Models/PlayingCards/Heart/SM_PC01h.SM_PC01h")))
    (:then_1
      (bind _output_get_41 (Variables|Default|SetH2 "/Game/Casino/Models/PlayingCards/Heart/SM_PC02h.SM_PC02h")))
    (:then_2
      (bind _output_get_42 (Variables|Default|SetH3 "/Game/Casino/Models/PlayingCards/Heart/SM_PC03h.SM_PC03h")))
    (:then_3
      (bind _output_get_43 (Variables|Default|SetH4 "/Game/Casino/Models/PlayingCards/Heart/SM_PC04h.SM_PC04h")))
    (:then_4
      (bind _output_get_44 (Variables|Default|SetH5 "/Game/Casino/Models/PlayingCards/Heart/SM_PC05h.SM_PC05h")))
    (:then_5
      (bind _output_get_45 (Variables|Default|SetH6 "/Game/Casino/Models/PlayingCards/Heart/SM_PC06h.SM_PC06h")))
    (:then_6
      (bind _output_get_46 (Variables|Default|SetH7 "/Game/Casino/Models/PlayingCards/Heart/SM_PC07h.SM_PC07h")))
    (:then_7
      (bind _output_get_47 (Variables|Default|SetH8 "/Game/Casino/Models/PlayingCards/Heart/SM_PC08h.SM_PC08h")))
    (:then_8
      (bind _output_get_48 (Variables|Default|SetH9 "/Game/Casino/Models/PlayingCards/Heart/SM_PC09h.SM_PC09h")))
    (:then_9
      (bind _output_get_49 (Variables|Default|SetH10 "/Game/Casino/Models/PlayingCards/Heart/SM_PC10h.SM_PC10h")))
    (:then_10
      (bind _output_get_50 (Variables|Default|SetHJ "/Game/Casino/Models/PlayingCards/Heart/SM_PC11h.SM_PC11h")))
    (:then_11
      (bind _output_get_51 (Variables|Default|SetHQ "/Game/Casino/Models/PlayingCards/Heart/SM_PC12h.SM_PC12h")))
    (:then_12
      (bind _output_get_52 (Variables|Default|SetHK "/Game/Casino/Models/PlayingCards/Heart/SM_PC13h.SM_PC13h"))))
  (Variables|Default|SetH (Utilities|Array|MakeArray _output_get_40 _output_get_41 _output_get_42 _output_get_43 _output_get_44 _output_get_45 _output_get_46 _output_get_47 _output_get_48 _output_get_49 _output_get_50 _output_get_51 _output_get_52))
  (Variables|Default|SetCards (Utilities|Array|MakeArray 0 1 2 3)))