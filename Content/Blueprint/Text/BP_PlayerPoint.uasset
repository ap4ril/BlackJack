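; BP_PlayerPoint is an actor that displays the game mode's Player value as text in the world.
; On BeginPlay it caches BP_GameModeBase, hides itself, then reappears after a fixed delay of about eight seconds.
; Every Tick it converts the game mode's Player integer to text and sets it on its TextRender component.
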(event EventBeginPlay
  (bind _asbp_game_mode_base (Utilities|Casting|CastToBP_GameModeBase (Game|GetGameMode)))
  (Variables|Default|SetGameMode _asbp_game_mode_base)
  (Rendering|SetActorHiddenInGame true)
  (Utilities|FlowControl|Delay 8.1)
  (Rendering|SetActorHiddenInGame false))

(event Collision|EventActorBeginOverlap
  (params (OtherActor :type Actor%20Object%20Reference)))

(event EventTick
  (params (DeltaSeconds :type Float%20%28single-precision%29))
  (Rendering|Components|TextRender|SetText (Variables|Default|GetTextRender) (Utilities|Text|ToText(Integer) (Variables|/Game/Blueprint/Gameplay/BP_GameModeBase.BP_GameModeBase_C|GetPlayer (Variables|Default|GetGameMode)))))

(fn ConstructionScript)