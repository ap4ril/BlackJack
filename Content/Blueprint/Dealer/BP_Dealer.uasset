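; Blackjack dealer actor that animates dealing, hit and stand actions and presents each round's result.
; Opens with a bow and deal, then polls GameMode flags on Tick to pick montages or show win/lose/draw and reload the level.
; MoveDeck macros time hand-held deck visibility and an IsServing flag to the animations.
; Standing moves BP_Deck via timeline and raises staggered Circle flags.
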(event Custom|Set
  (bind _asbp_game_mode_base (Utilities|Casting|CastToBP_GameModeBase (Game|GetGameMode)))
  (Variables|Default|SetGamemode _asbp_game_mode_base))

(event Custom|Play2
  (Variables|/Game/Blueprint/Gameplay/BP_GameModeBase.BP_GameModeBase_C|SetHitPressed (Variables|Default|GetGamemode) false)
  (Animation|Montage|PlayMontage (Variables|Default|GetDealer) "/Game/Animation/Cards2_Montage.Cards2_Montage"
    (:then
      (|MoveDeck_2))))

(event Custom|Stand
  (bind _deck (Variables|Default|GetDeck))
  (Variables|/Game/Blueprint/Gameplay/BP_GameModeBase.BP_GameModeBase_C|SetStandPressed (Variables|Default|GetGamemode) false)
  (Animation|Montage|PlayMontage (Variables|Default|GetDealer) "/Game/Animation/Thankful__1__Montage.Thankful__1__Montage"
    (:OnCompleted
      (Animation|Montage|PlayMontage (Variables|Default|GetDealer) "/Game/Animation/Hands_Forward_Gesture_Montage.Hands_Forward_Gesture_Montage"
        (:then
          (Utilities|FlowControl|Delay 0.3)
          (bind _alpha (Timeline|타임라인_0 Play)
            (:Update
              (Transformation|SetActorLocation _deck (Math|Vector|Lerp(Vector) "-40.000000,-25.000000,116.000000" "3.000000,-28.000000,145.000000" _alpha) false false)
              (Transformation|SetActorRotation _deck (Math|Rotator|Lerp(Rotator) "0, 0, 0" "0, 0,90.000000" _alpha))
              (Utilities|FlowControl|Delay 0.5)
              (Variables|Default|SetCircle true)
              (Utilities|FlowControl|Delay 0.2)
              (Variables|Default|SetCircle1 true)
              (Utilities|FlowControl|Delay 0.2)
              (Variables|Default|SetCircle2 true)
              (Utilities|FlowControl|Delay 0.2)
              (Variables|Default|SetCircle3 true)
              (Utilities|FlowControl|Delay 0.2)
              (Variables|Default|SetCircle4 true)
              (Utilities|FlowControl|Delay 0.2)
              (Variables|Default|SetCircle5 true)
              (Utilities|FlowControl|Delay 0.2)
              (Variables|Default|SetCircle6 true)
              (Utilities|FlowControl|Delay 0.2)
              (Variables|Default|SetCircle7 true))))))))

(event EventBeginPlay
  (bind _returnvalue (Actor|GetActorOfClass "/Game/Blueprint/Card/BP_Deck.BP_Deck_C"))
  (Variables|Default|SetDeck _returnvalue)
  (Utilities|FlowControl|Delay 1.0)
  (Animation|Montage|PlayMontage (Variables|Default|GetDealer) "/Game/Animation/Quick_Formal_Bow_Montage.Quick_Formal_Bow_Montage" 1.5
    (:OnCompleted
      (Utilities|FlowControl|Delay 0.1)
      (Animation|Montage|PlayMontage (Variables|Default|GetDealer) "/Game/Animation/Cards_Montage.Cards_Montage"
        (:then
          (|MoveDeck))))))

(event Collision|EventActorBeginOverlap
  (params (OtherActor :type Actor%20Object%20Reference)))

(event EventTick
  (params (DeltaSeconds :type Float%20%28single-precision%29))
  (CallFunction|Set)
  (if (Variables|/Game/Blueprint/Gameplay/BP_GameModeBase.BP_GameModeBase_C|GetHitPressed (Variables|Default|GetGamemode))
    (CallFunction|Play2)
    (elif (Variables|/Game/Blueprint/Gameplay/BP_GameModeBase.BP_GameModeBase_C|GetWin (Variables|Default|GetGamemode))
      (Variables|/Game/Blueprint/Gameplay/BP_GameModeBase.BP_GameModeBase_C|SetWin (Variables|Default|GetGamemode) false)
      (Utilities|FlowControl|Delay 3.0)
      (Widget|SetVisibility (Variables|/Game/Blueprint/Gameplay/BP_GameModeBase.BP_GameModeBase_C|GetYouWin (Variables|Default|GetGamemode)) "Visible")
      (Rendering|SetVisibility (Variables|/Game/Blueprint/Card/BP_Deck.BP_Deck_C|GetDeck (Variables|Default|GetDeck)) false false)
      (Utilities|FlowControl|Delay 0.5)
      (Transformation|SetActorLocation self "0,-96.000000,20.000000" false false)
      (Animation|Montage|PlayMontage (Variables|Default|GetDealer) "/Game/Animation/Clapping.Clapping"
        (:OnCompleted
          (Game|OpenLevel(byName) "Blackjack")))
      (elif (Variables|/Game/Blueprint/Gameplay/BP_GameModeBase.BP_GameModeBase_C|GetLose (Variables|Default|GetGamemode))
        (Variables|/Game/Blueprint/Gameplay/BP_GameModeBase.BP_GameModeBase_C|SetLose (Variables|Default|GetGamemode) false)
        (Utilities|FlowControl|Delay 4.5)
        (Widget|SetVisibility (Variables|/Game/Blueprint/Gameplay/BP_GameModeBase.BP_GameModeBase_C|GetYouLose (Variables|Default|GetGamemode)) "Visible")
        (Rendering|SetVisibility (Variables|/Game/Blueprint/Card/BP_Deck.BP_Deck_C|GetDeck (Variables|Default|GetDeck)) false false)
        (Animation|Montage|PlayMontage (Variables|Default|GetDealer) "/Game/Animation/Quick_Formal_Bow_Montage.Quick_Formal_Bow_Montage"
          (:then
            (Utilities|FlowControl|Delay 3.5)
            (Game|OpenLevel(byName) "Blackjack")))
        (elif (Variables|/Game/Blueprint/Gameplay/BP_GameModeBase.BP_GameModeBase_C|GetDraw (Variables|Default|GetGamemode))
          (Utilities|FlowControl|Delay 5.5)
          (Widget|SetVisibility (Variables|/Game/Blueprint/Gameplay/BP_GameModeBase.BP_GameModeBase_C|GetYouDraw (Variables|Default|GetGamemode)) "Visible")
          (Rendering|SetVisibility (Variables|/Game/Blueprint/Card/BP_Deck.BP_Deck_C|GetDeck (Variables|Default|GetDeck)) false false)
          (Variables|/Game/Blueprint/Gameplay/BP_GameModeBase.BP_GameModeBase_C|SetDraw (Variables|Default|GetGamemode) false)
          (Utilities|FlowControl|Delay 1.5)
          (Game|OpenLevel(byName) "Blackjack")
          (elif (Variables|/Game/Blueprint/Gameplay/BP_GameModeBase.BP_GameModeBase_C|GetStandPressed (Variables|Default|GetGamemode))
            (CallFunction|Stand)))))))

(fn ConstructionScript)